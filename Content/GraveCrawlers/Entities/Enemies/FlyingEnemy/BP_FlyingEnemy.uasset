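; Flying enemy Blueprint that fires projectiles at the player and grants XP to its killer on death.
; Attacks glow red through an emissive timeline, then launch a projectile with a computed speed toward a randomly offset player position.
; Death stops movement, plays a material disintegration, then spawns an XP pickup immediately collected by the killer.
; Damage shows a camera-oriented health bar and restarts its one-second timer.
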(event EventBeginPlay
  (bind _aswbp_health_bar (Utilities|Casting|CastToWBP_HealthBar (UserInterface|GetWidget (Variables|Default|GetHealthBarWidget))))
  (Variables|Default|SetHealthBarWidgetBP _aswbp_health_bar)
  (|CallParentFunction))

(event Collision|EventActorBeginOverlap
  (params (OtherActor :type Actor%20Object%20Reference)))

(event EventTick
  (params (DeltaSeconds :type Float%20%28single-precision%29)))

(event EventOnDeath
  (params (KillingActor :type Actor%20Object%20Reference))
  (bind _pathagentcomponent (Variables|Default|GetPathAgentComponent))
  (bind _mesh (Variables|Character|GetMesh))
  ;[0.15 0.15 0.15 0.5] OnDeath - Disintegrate animation and XP
  (Class|GC3DPathFindingAgent|StopMovement _pathagentcomponent)
  (Class|GC3DPathFindingAgent|DisableMovement _pathagentcomponent)
  (Class|FlyingEnemy|SetCurrentState "Stateless")
  (bind _returnvalue (Rendering|Material|CreateDynamicMaterialInstance _mesh 0 0 "None" :!class /Script/Engine.PrimitiveComponent))
  (bind _returnvalue_2 (Rendering|Material|CreateDynamicMaterialInstance _mesh 1 0 "None" :!class /Script/Engine.PrimitiveComponent))
  (bind _desintegrate_progress (Timeline|Timeline Play)
    (:Update
      (Rendering|Material|SetScalarParameterValue _returnvalue "Amount" _desintegrate_progress :!class /Script/Engine.MaterialInstanceDynamic))
    (:Finished
      (|CallParentFunction KillingActor)
      (CallFunction|HideHealthBar)
      (bind _returnvalue_3 (Game|SpawnActorfromClass "/Game/GraveCrawlers/Blueprints/BP_EXPPickup.BP_EXPPickup_C" (Math|Transform|MakeTransform (Transformation|GetActorLocation) "0, 0, 0" "1.000000,1.000000,1.000000") "Undefined" "MultiplyWithRoot" 0 0))
      (Default|Drop _returnvalue_3 (Math|Random|RandomFloatinRange 0.0 (Variables|/Script/Prototype1.EnemyDataAsset|GetExpDropMax (Variables|Default|GetEnemyConfig))))
      (Default|Pickup _returnvalue_3 KillingActor)
      (|CallParentFunction))))

(event EventStartAttack
  (bind _attackpoint (Variables|Default|GetAttackPoint))
  (bind _mesh (Variables|Character|GetMesh))
  (bind _mesh_2 (Variables|Character|GetMesh))
  (bind _returnvalue (Transformation|GetWorldTransform _attackpoint))
  (Variables|Default|SetIsAttacking true)
  (Rendering|Material|SetColorParameterValueonMaterials _mesh_2 "EmissiveFactor" "(R=1.000000,G=0.000000,B=0.000000,A=1.000000)")
  (bind _emissivestr (Timeline|ColourTimeline PlayFromStart)
    (:Update
      (Rendering|Material|SetScalarParameterValueonMaterials _mesh_2 "EmissiveStrength" _emissivestr))
    (:Finished
      (bind _returnvalue_2 (Game|SpawnActorfromClass "/Game/GraveCrawlers/Entities/Enemies/FlyingEnemy/BP_FlyingEnemyProjectile.BP_FlyingEnemyProjectile_C" (Math|Transform|MakeTransform (.location _returnvalue) (.rotation _returnvalue) "1.000000,1.000000,1.000000") "Undefined" "MultiplyWithRoot" 0 self))
      (Class|FlyingEnemyProjectile|Initialize _returnvalue_2 (Variables|Default|GetDamage))
      (bind _targetplayer (Variables|Default|GetTargetPlayer)
        (:then
          (bind _returnvalue_3 (Class|GCUtilities|CalculateInitialVelocitytoReachPoint (.location _returnvalue) (+ (Transformation|GetActorLocation _targetplayer) (* (Math|Random|RandomUnitVector) (Variables|Default|GetAttackErrorRadius))) 0.0))
          (Variables|/Script/Engine.MovementComponent|SetVelocity (Variables|/Script/Prototype1.ShooterProjectile|GetProjectileMovement _returnvalue_2) (* (Math|Vector|GetForwardVector (.rotation _returnvalue)) _returnvalue_3))
          (Rendering|Material|SetColorParameterValueonMaterials _mesh "EmissiveFactor" "(R=1.000000,G=1.000000,B=1.000000,A=1.000000)")
          (Rendering|Material|SetScalarParameterValueonMaterials _mesh "EmissiveStrength" 1.0)
          (|CallParentFunction))
        (:else
          (Development|PrintString "NNo player"))))))

(fn ConstructionScript)

(fn OnDamaged
  (bind (_current _max) (Class|HealthComponent|GetCurrentandMaxHealth (Variables|Default|GetHealthComponent)))
  (CallFunction|ShowHealthBar)
  (bind _healthbarwidgetbp (Variables|Default|GetHealthBarWidgetBP)
    (:then
      (Progress|SetPercent (Variables|/Game/GraveCrawlers/UI/WBP_HealthBar.WBP_HealthBar_C|GetHealthBar _healthbarwidgetbp) (Math|Float|SafeDivide _current _max))
      (CallFunction|OrientHealthBartoScreen)
      (Utilities|Time|ClearandInvalidateTimerbyHandle (Variables|Default|GetShowHealthBarTimer))
      (bind _returnvalue (Utilities|Time|SetTimerbyEvent (EventDispatchers|CreateEvent :!event HideHealthBar) 1.0))
      (Variables|Default|SetShowHealthBarTimer _returnvalue))
    (:else
      (Development|PrintString "Invalid"))))

(fn OrientHealthBartoScreen
  (bind _healthbarwidget (Variables|Default|GetHealthBarWidget))
  (Transformation|SetWorldRotation _healthbarwidget (Math|Rotator|FindLookatRotation (Transformation|GetWorldLocation _healthbarwidget) (Camera|GetCameraLocation (Game|GetPlayerCameraManager 0))) false false))

(fn ShowHealthBar
  (bind _healthbarwidget (Variables|Default|GetHealthBarWidget))
  (Rendering|SetVisibility _healthbarwidget true false)
  (Class|WidgetComponent|SetTickMode _healthbarwidget "Enabled"))

(fn HideHealthBar
  (bind _healthbarwidget (Variables|Default|GetHealthBarWidget))
  (Rendering|SetVisibility _healthbarwidget false false)
  (Class|WidgetComponent|SetTickMode _healthbarwidget "Disabled"))