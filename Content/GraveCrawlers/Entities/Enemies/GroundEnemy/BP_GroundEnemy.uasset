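; Melee ground enemy that damages the main character and hands its target to a basic-enemy AI controller's behaviour tree.
; Attack triggers the AnimBP attack, swaps in a weapon attack material and starts a cooldown timer.
; AnimBP attack start/end events toggle the hit trigger's overlaps, while CanDamage stops repeat hits after damage lands.
; Death disables attacking, and attack-speed stat changes pass to the AnimBP.
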(event OnComponentBeginOverlap(AttackingTrigger)
  (params (OverlappedComponent :type Primitive%20Component%20Object%20Reference) (OtherActor :type Actor%20Object%20Reference) (OtherComp :type Primitive%20Component%20Object%20Reference) (OtherBodyIndex :type Integer) (bFromSweep :type Boolean) (SweepResult :type Hit%20Result%20Structure%20%28by%20ref%29))
  (if (Variables|Default|GetCanDamage)
    (bind _asbp_main_char (Utilities|Casting|CastToBP_MainChar OtherActor))
    (Default|DealDamage (Variables|/Game/GraveCrawlers/Entities/Character/BP_MainChar.BP_MainChar_C|GetHealthComponent%20 _asbp_main_char) (Variables|Default|GetDamage) 0)
    (Variables|Default|SetCanDamage false)))

(event EventBeginPlay
  (|CallParentFunction)
  (bind _asabp_base_ground_enemy (Utilities|Casting|CastToABP_BaseGroundEnemy (Components|SkeletalMesh|GetAnimInstance (Variables|Character|GetMesh))))
  (EventDispatchers|BindEventtoAnimAttackStarted _asabp_base_ground_enemy (EventDispatchers|CreateEvent :!event AnimationHitStarted))
  (EventDispatchers|BindEventtoAnimAttackEnded _asabp_base_ground_enemy (EventDispatchers|CreateEvent :!event AnimationHitEnded))
  (Variables|Default|SetMaskVariable (Variables|Default|GetEnemyMask)))

(event EventOnDeath
  (params (KillingActor :type Actor%20Object%20Reference))
  (Utilities|Time|ClearandInvalidateTimerbyHandle (Variables|Default|GetAttackTimerHandle))
  (Variables|Default|SetCanAttack false)
  (Variables|Default|SetCanDamage false)
  (|CallParentFunction KillingActor))

(fn ConstructionScript
  (|CallParentFunction))

(fn SetCanAttack
  (Variables|Default|SetCanAttack true)
  (Variables|Default|SetCanDamage true))

(fn Attack
  (if (Variables|Default|GetCanAttack)
    (bind _asabp_base_ground_enemy (Utilities|Casting|CastToABP_BaseGroundEnemy (Components|SkeletalMesh|GetAnimInstance (Variables|Character|GetMesh))))
    (Default|Attack _asabp_base_ground_enemy)
    (Rendering|Material|SetMaterial (Variables|Character|GetMesh) 1 (Variables|Default|GetWeaponAttackMaterial))
    (Variables|Default|SetCanAttack false)
    (bind _returnvalue (Utilities|Time|SetTimerbyEvent (EventDispatchers|CreateEvent :!event SetCanAttack) (Variables|Default|GetAttackCooldown)))
    (Variables|Default|SetAttackTimerHandle _returnvalue)))

(fn SetTarget
  (params (TargetActor :type Actor%20Object%20Reference))
  (bind _asaic_basic_enemy (Utilities|Casting|CastToAIC_BasicEnemy (AI|GetAIController self)))
  (Default|StartBehaviourTree _asaic_basic_enemy TargetActor))

(fn AnimationHitStarted
  (Variables|/Script/Engine.PrimitiveComponent|SetbGenerateOverlapEvents (Variables|Default|GetAttackingTrigger) true)
  (Audio|PlaySoundatLocation "/Game/GraveCrawlers/Audio/Sounds/SkeletonAttack/SW_EnemyAttack.SW_EnemyAttack" (Transformation|GetActorLocation) "0, 0, 0" 1.0 1.0 0.0 "/Game/GraveCrawlers/Audio/Sounds/others/EnemyAttenuation.EnemyAttenuation" 0 0 0))

(fn AnimationHitEnded
  (Variables|/Script/Engine.PrimitiveComponent|SetbGenerateOverlapEvents (Variables|Default|GetAttackingTrigger) false)
  (Rendering|Material|SetMaterial (Variables|Character|GetMesh) 1 "/Game/GraveCrawlers/Entities/Enemies/GroundEnemy/Materials/M_Skin_Skeleton.M_Skin_Skeleton"))

(fn AttackSpeedStatChanged
  (params (Current :type Float%20%28single-precision%29))
  (bind _asabp_base_ground_enemy (Utilities|Casting|CastToABP_BaseGroundEnemy (Components|SkeletalMesh|GetAnimInstance (Variables|Character|GetMesh))))
  (Default|SetAttackSpeed _asabp_base_ground_enemy Current))

(fn StopAbilitytoAttack
  (Utilities|Time|ClearandInvalidateTimerbyHandle (Variables|Default|GetAttackTimerHandle))
  (Variables|Default|SetCanAttack false)
  (Variables|Default|SetCanDamage false)
  (Rendering|Material|SetMaterial (Variables|Character|GetMesh) 1 "/Game/GraveCrawlers/Entities/Enemies/GroundEnemy/Materials/M_Skin_Skeleton.M_Skin_Skeleton"))