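; Base ground enemy Blueprint that adds health bar feedback, a disintegration death effect and experience drops.
; Taking damage reveals the widget health bar, updates its percent, rotates it toward the player camera and restarts a one-second timer.
; Death stops movement and runs a timeline driving dynamic material parameters on mesh and mask.
; When it finishes, the bar hides, a randomized XP pickup drops and parent death logic completes.
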(event EventBeginPlay
  (bind _aswbp_health_bar (Utilities|Casting|CastToWBP_HealthBar (UserInterface|GetWidget (Variables|Default|GetHealthBar))))
  (Variables|Default|SetHealthBarAsWidgetClass _aswbp_health_bar)
  (|CallParentFunction))

(event EventOnDeath
  (params (KillingActor :type Actor%20Object%20Reference))
  (bind _movementcomponent (Variables|Default|GetMovementComponent))
  (bind _enemyconfig (Variables|Default|GetEnemyConfig))
  (bind _mesh (Variables|Character|GetMesh))
  (bind _maskvariable (Variables|Default|GetMaskVariable))
  ;[0.15 0.15 0.15 0.5] OnDeath - Disintegrate animation and XP
  (Components|Movement|StopMovementImmediately _movementcomponent)
  (Components|Activation|Deactivate _movementcomponent)
  (Rendering|Material|SetMaterial _maskvariable 0 (Rendering|Material|GetMaterial (Variables|Character|GetMesh) 0))
  (bind _returnvalue (Rendering|Material|CreateDynamicMaterialInstance _maskvariable 0 0 "None" :!class /Script/Engine.PrimitiveComponent))
  (bind _returnvalue_2 (Rendering|Material|CreateDynamicMaterialInstance _mesh 0 0 "None" :!class /Script/Engine.PrimitiveComponent))
  (bind _returnvalue_3 (Rendering|Material|CreateDynamicMaterialInstance _mesh 1 0 "None" :!class /Script/Engine.PrimitiveComponent))
  (bind _desintegrate_progress (Timeline|Timeline Play)
    (:Update
      (Rendering|Material|SetScalarParameterValue _returnvalue_2 "Amount" _desintegrate_progress :!class /Script/Engine.MaterialInstanceDynamic))
    (:Finished
      (|CallParentFunction KillingActor)
      (CallFunction|HideHealthBar)
      (bind _returnvalue_4 (Game|SpawnActorfromClass "/Game/GraveCrawlers/Blueprints/BP_EXPPickup.BP_EXPPickup_C" (Math|Transform|MakeTransform (Transformation|GetActorLocation) "0, 0, 0" "1.000000,1.000000,1.000000") "Undefined" "MultiplyWithRoot" 0 0))
      (Default|Drop _returnvalue_4 (Math|Random|RandomFloatinRange (Variables|/Script/Prototype1.EnemyDataAsset|GetExpDropMin _enemyconfig) (Variables|/Script/Prototype1.EnemyDataAsset|GetExpDropMax _enemyconfig)))
      (|CallParentFunction))))

(event EventOnHealthManipulated
  (|CallParentFunction)
  (bind (_current _max) (Class|HealthComponent|GetCurrentandMaxHealth (Variables|Default|GetHealthComponent)))
  (if (> _max 0.0)
    (bind _healthbaraswidgetclass (Variables|Default|GetHealthBarAsWidgetClass)
      (:then
        (Progress|SetPercent (Variables|/Game/GraveCrawlers/UI/WBP_HealthBar.WBP_HealthBar_C|GetHealthBar _healthbaraswidgetclass) (/ _current _max)))
      (:else
        (Development|PrintString "Invalid")))))

(fn ConstructionScript)

(fn HealthStatChanged
  (params (Current :type Float%20%28single-precision%29) (Max :type Float%20%28single-precision%29))
  (|CallParentFunction Current Max))

(fn OrientHealthBartoScreen
  (bind _healthbar (Variables|Default|GetHealthBar))
  (Transformation|SetWorldRotation _healthbar (Math|Rotator|FindLookatRotation (Transformation|GetWorldLocation _healthbar) (Camera|GetCameraLocation (Game|GetPlayerCameraManager 0))) false false))

(fn OnDamaged
  (bind (_current _max) (Class|HealthComponent|GetCurrentandMaxHealth (Variables|Default|GetHealthComponent)))
  (CallFunction|ShowHealthBar)
  (bind _healthbaraswidgetclass (Variables|Default|GetHealthBarAsWidgetClass)
    (:then
      (Progress|SetPercent (Variables|/Game/GraveCrawlers/UI/WBP_HealthBar.WBP_HealthBar_C|GetHealthBar _healthbaraswidgetclass) (Math|Float|SafeDivide _current _max))
      (CallFunction|OrientHealthBartoScreen)
      (Utilities|Time|ClearandInvalidateTimerbyHandle (Variables|Default|GetShowHealthBarTimer))
      (bind _returnvalue (Utilities|Time|SetTimerbyEvent (EventDispatchers|CreateEvent :!event HideHealthBar) 1.0))
      (Variables|Default|SetShowHealthBarTimer _returnvalue))
    (:else
      (Development|PrintString "Invalid"))))

(fn ShowHealthBar
  (bind _healthbar (Variables|Default|GetHealthBar))
  (Rendering|SetVisibility _healthbar true false)
  (Class|WidgetComponent|SetTickMode _healthbar "Enabled"))

(fn HideHealthBar
  (bind _healthbar (Variables|Default|GetHealthBar))
  (Rendering|SetVisibility _healthbar false false)
  (Class|WidgetComponent|SetTickMode _healthbar "Disabled"))