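; BP_AIManager is an enemy spawner that binds to the main game mode's first-mode and second-mode change events.
; SpawnEnemiesRandom loops on a wave budget, spawning pawns with random spread around shuffled spawn points, within concurrent-enemy and attempt limits.
; Enemy tracking, second-mode stat changes and cost-based budget deduction are disconnected, so successful spawns never reduce the budget.
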(event EventBeginPlay
  (bind _asbp_main_game_mode (Utilities|Casting|CastToBP_MainGameMode (Game|GetGameMode)))
  (EventDispatchers|BindEventtoOnChangedtoFirstMode _asbp_main_game_mode (EventDispatchers|CreateEvent :!event OnChangedtoFirstMode))
  (EventDispatchers|BindEventtoOnChangedtoSecondMode _asbp_main_game_mode (EventDispatchers|CreateEvent :!event OnChangedtoSecondMode)))

(fn ConstructionScript)

(fn SpawnEnemiesRandom
  (params (Count :type Integer) (Type :type Pawn%20Class%20Reference) (Location :type BP%20AI%20Spawn%20Point%20Object%20Reference))
  (LocalVariables|SetWaveBudget Count)
  (while (and (> (LocalVariables|GetWaveBudget) 0) (LocalVariables|GetSpawningSuccessfully))
    (bind _spawnpointout (CallFunction|GetRandomSpawnPoint))
    (if (< (Utilities|Array|Length (Variables|Default|GetBaseEnemiesInScene)) (Variables|Default|GetMaxEnemies))
      (if (< (LocalVariables|GetIterations) (LocalVariables|GetMaxIterations))
        (bind _returnvalue (AI|SpawnAIFromClass Type 0 (+ (Transformation|GetActorLocation _spawnpointout) (* (Math|Random|RandomUnitVector) (Variables|Default|GetSpawnSpread))) "0, 0, 0" false 0))
        (Utilities|IsValid _returnvalue
          (:Is%20Valid
            (bind _asbp_ground_enemy_base (Utilities|Casting|CastToBP_GroundEnemyBase _returnvalue)))
          (:Is%20Not%20Valid
            (Math|Integer|IncrementInt (LocalVariables|GetIterations))))
        (else
          (Development|PrintString "AIMANAGER:: Max enemy spawn attempts reached.")
          (LocalVariables|SetSpawningSuccessfully false)))
      (else
        (Development|PrintString "AIMANAGER::Max Concurrent enemies reached.")
        (LocalVariables|SetSpawningSuccessfully false))))
  (return (LocalVariables|GetSpawningSuccessfully)))

(fn GetRandomSpawnPoint
  (bind _spawnpositions (Variables|Default|GetSpawnPositions))
  (Utilities|Array|Shuffle _spawnpositions)
  (return (Utilities|Array|Get(acopy) _spawnpositions)))