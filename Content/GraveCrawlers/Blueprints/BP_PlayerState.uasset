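; Player state for GraveCrawlers that tracks experience, level, pickup radius and an enum-keyed stat set.
; GiveEXP banks XP and starts a fast looping timer whose IncrementEXP ticks the displayed value up, levelling up at the threshold and firing dispatchers.
; A separate GiveXP event does similar counting with a Delay loop.
; Stat functions read map entries and write current values capped at each stat's maximum.
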(event Custom|GiveXP
  (params (EXPAmount :type Integer))
  (bind _variable (|TemporaryVariable))
  (|Assign _variable 1)
  (if (<= _variable EXPAmount) :!label _label
    (Utilities|FlowControl|Sequence
      (:then_0
        (bind _result (Math|Integer|IncrementInt (Variables|Default|GetCurrentEXP))
          (:%20%20
            (if (>= _result (Variables|Default|GetEXPToLevelUp))
              (Variables|Default|SetCurrentEXP 0)
              (Math|Integer|IncrementInt (Variables|Default|GetLevel)
                (:%20%20
                  _)))
            (Default|CallOnEXPChanged))))
      (:then_1
        (|Assign _variable (+ _variable 1))
        (Utilities|FlowControl|Delay 0.1)
        (goto _label)))))

(event EventBeginPlay)

(event EventTick
  (params (DeltaSeconds :type Float%20%28single-precision%29)))

(fn ConstructionScript)

(fn GiveEXP
  (params (EXPAmount :type Integer))
  (bind _output_get (Variables|Default|SetEXPToBeAdded EXPAmount))
  (Variables|Default|SetCurrentEXP (+ _output_get (Variables|Default|GetCurrentEXP)))
  (if (not (Utilities|Time|IsTimerActivebyHandle (Variables|Default|GetEXPIncrementingHandle)))
    (bind _returnvalue (Utilities|Time|SetTimerbyFunctionName 0 "IncrementEXP" 0.005 true))
    (Variables|Default|SetEXPIncrementingHandle _returnvalue)))

(fn IncrementEXP
  (Math|Integer|IncrementInt (Variables|Default|GetIncrementingEXP)
    (:%20%20
      (bind _result (Math|Integer|IncrementInt (Variables|Default|GetEXPToDisplay))
        (:%20%20
          (if (>= _result (Variables|Default|GetEXPToLevelUp))
            (Variables|Default|SetEXPToDisplay 0)
            (Math|Integer|IncrementInt (Variables|Default|GetLevel)
              (:%20%20
                (Default|CallOnLevelChanged))))
          (Default|CallOnEXPChanged)
          (if (>= (Variables|Default|GetIncrementingEXP) (Variables|Default|GetCurrentEXP))
            (Utilities|Time|ClearandInvalidateTimerbyHandle (Variables|Default|GetEXPIncrementingHandle))))))))

(fn ChangePickupRadius
  (params (New%20Radius :type Float%20%28double-precision%29))
  (Variables|Default|SetPickupRadius New%20Radius)
  (Default|CallOnPickupRadiusChanged))

(fn Initialize)

(fn GetStatValues
  (params (Type :type E_StatTypes%20Enum :default "NewEnumerator4"))
  (bind _statset (Variables|Default|GetStatSet))
  (bind (_value _returnvalue) (Utilities|Map|Find _statset Type))
  (if _returnvalue
    (return (.startamount _value) (.maxamount _value) (.currentamount _value) true)
    (else
      (Development|PrintString "Unable to find stat set by enum type.")
      (return 0.0 0.0 0.0 false))))

(fn InputStatCurrent
  (params (Type :type E_StatTypes%20Enum :default "NewEnumerator4") (Amount :type Float%20%28double-precision%29))
  (bind _statset (Variables|Default|GetStatSet))
  (bind (_value _returnvalue) (Utilities|Map|Find _statset Type))
  (bind _returnvalue_2 (Math|Float|Min(Float) Amount (.maxamount _value)))
  (if _returnvalue
    (Utilities|Map|Add _statset (.type _value) (Utilities|Struct|MakeS_PlayerStat (.type _value) (.startamount _value) (.maxamount _value) _returnvalue_2))
    (return _returnvalue_2 true)
    (else
      (return 0.0 false))))

(fn InputStatwithSeparateCurrentandMaxIntoSet
  (params (Type :type E_StatTypes%20Enum :default "NewEnumerator4") (CurrentAmount :type Float%20%28double-precision%29) (MaxAmount :type Float%20%28double-precision%29))
  (bind _statset (Variables|Default|GetStatSet))
  (bind (_value _returnvalue) (Utilities|Map|Find _statset Type))
  (if _returnvalue
    (bind (_currentout _maxout) (|ClampValues CurrentAmount MaxAmount (.maxamount _value)))
    (Utilities|Map|Add _statset Type (Utilities|Struct|MakeS_PlayerStat Type (.startamount _value) (.maxamount _value) _currentout))
    (return _currentout _maxout true)
    (else
      (Development|PrintString "INPUT_STAT_CURRENT_MAX_IN_ST::Could not find stat type in stat set.")
      (return 0.0 0.0 false))))