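; Ability component for the main character that throws an object which spawns a slow area where it lands.
; On begin play it creates a hand-socketed throwable mesh and a preview mesh from its data asset.
; Using the ability starts a looping timer that places the preview at the predicted projectile endpoint along the camera aim.
; Confirming launches the throwable and starts cooldown; landing spawns BP_SlowAbility using owner radius, slow and duration stats.
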(event EventBeginPlay
  ;[0.15 0.15 0.15 0.5] Start
  (bind _asbp_main_char (Utilities|Casting|CastToBP_MainChar (Components|GetOwner)))
  (bind _output_get (Variables|Default|SetOwningPlayer _asbp_main_char))
  (bind _aspda_slow_ability (Utilities|Casting|CastToPDA_SlowAbility (Variables|Default|GetAbilityDA)))
  (bind _output_get_2 (Variables|Default|SetSlowAbilityDataAsset _aspda_slow_ability))
  (|InitAbilityComponents _output_get _output_get_2))

(event EventUseAbility
  ;[0.15 0.15 0.15 0.5] Use Ability
  (|CallParentFunction)
  (if (not (Variables|Default|GetOnCooldown))
    (bind _owningplayer (Variables|Default|GetOwningPlayer)
      (:then
        (bind _asbpi_thrower (Utilities|Casting|CastToBPI_Thrower _owningplayer))
        (Rendering|SetVisibility (Variables|Default|GetThrowingComponent) true false)
        (Default|StartThrow _asbpi_thrower)
        (CallFunction|StartDisplayingAbilityBlueprint))
      (:else))))

(event EventOnAbilityStatChanged
  (params (tag :type Gameplay%20Tag%20Structure) (stats :type Runtime%20Stats%20Structure))
  ;[0.15 0.15 0.15 0.5] On Ability Stats Changed
  (|SwitchGameplayTag tag
    (:Stats.Ability.SlowArea.Radius
      (Transformation|SetRelativeScale3D (Variables|Default|GetAbilityPreviewObject) (Math|Vector|MakeVector (.currentvalue stats) (.currentvalue stats) 1.0)))))

(event EventCancelAbility
  ;[0.15 0.15 0.15 0.5] Cancel Ability
  (|CallParentFunction)
  (Default|EndThrow (Variables|Default|GetOwningPlayer))
  (Rendering|SetVisibility (Variables|Default|GetAbilityPreviewObject) false false)
  (Rendering|SetVisibility (Variables|Default|GetThrowingComponent) false false)
  (Utilities|Time|ClearandInvalidateTimerbyHandle (Variables|Default|GetAbilityPreviewTimerHandle)))

(event EventConfirmAbility
  ;[0.15 0.15 0.15 0.5] Confirm Ability
  (|CallParentFunction)
  (if (not (Variables|Default|GetOnCooldown))
    (CallFunction|ThrowItem)
    (bind _owningplayer (Variables|Default|GetOwningPlayer)
      (:then
        (bind _asbpi_thrower (Utilities|Casting|CastToBPI_Thrower _owningplayer))
        (Default|EndThrow _asbpi_thrower)
        (bind _returnvalue (Class|Ability|StartCooldown))
        (if (not _returnvalue)
          (Development|PrintString "Failed to start cd")))
      (:else))))

(fn ThrowItem
  (bind _owningplayer (Variables|Default|GetOwningPlayer)
    (:then
      (bind _slowabilitydataasset (Variables|Default|GetSlowAbilityDataAsset)
        (:then
          (bind _returnvalue (Game|SpawnActorfromClass (Variables|/Game/GraveCrawlers/Data/Blueprints/PDA_SlowAbility.PDA_SlowAbility_C|GetThrowableObjectBlueprint _slowabilitydataasset) (Transformation|GetWorldTransform (Variables|Default|GetThrowingComponent)) "Undefined" "MultiplyWithRoot" 0 0))
          (Utilities|Time|ClearandInvalidateTimerbyHandle (Variables|Default|GetAbilityPreviewTimerHandle))
          (Rendering|SetVisibility (Variables|Default|GetThrowingComponent) false false)
          (Rendering|SetVisibility (Variables|Default|GetAbilityPreviewObject) false false)
          (Default|Launch _returnvalue (Math|Vector|GetForwardVector (Variables|/Game/GraveCrawlers/Entities/Character/BP_MainChar.BP_MainChar_C|GetFollowCamera _owningplayer)) (Variables|/Game/GraveCrawlers/Data/Blueprints/PDA_SlowAbility.PDA_SlowAbility_C|GetThrowForce _slowabilitydataasset) (Variables|/Game/GraveCrawlers/Data/Blueprints/PDA_SlowAbility.PDA_SlowAbility_C|GetThrowingMesh (Variables|Default|GetSlowAbilityDataAsset)))
          (EventDispatchers|BindEventtoOnLanded _returnvalue (EventDispatchers|CreateEvent :!event OnThrowableLanded)))
        (:else)))
    (:else)))

(fn ThrowFinished)

(fn OnThrowableLanded
  (params (Location :type Vector))
  (bind _ownerstatcomponent (Variables|Default|GetOwnerStatComponent))
  (bind _returnvalue (Game|SpawnActorfromClass "/Game/GraveCrawlers/Blueprints/Abilities/BP_SlowAbility.BP_SlowAbility_C" (Math|Transform|MakeTransform Location "0, 0, 0" "1.000000,1.000000,1.000000") "Undefined" "MultiplyWithRoot" 0 0))
  (bind _returnvalue_2 (Class|StatComponent|GetRuntimeStatSet _ownerstatcomponent "(TagName=\"Stats.Ability.SlowArea.Radius\")"))
  (bind _returnvalue_3 (Class|StatComponent|GetRuntimeStatSet _ownerstatcomponent "(TagName=\"Stats.Ability.SlowArea.SlowPercent\")"))
  (bind _returnvalue_4 (Class|StatComponent|GetRuntimeStatSet _ownerstatcomponent "(TagName=\"Stats.Ability.SlowArea.Duration\")"))
  (Default|Initialize _returnvalue (.currentvalue _returnvalue_2) (.currentvalue _returnvalue_3) (.currentvalue _returnvalue_4)))

(fn StartDisplayingAbilityBlueprint
  (Rendering|SetVisibility (Variables|Default|GetAbilityPreviewObject) true false)
  (bind _returnvalue (Utilities|Time|SetTimerbyEvent (EventDispatchers|CreateEvent :!event ShowAbilityPreview) 0.01 true))
  (Variables|Default|SetAbilityPreviewTimerHandle _returnvalue))

(fn ShowAbilityPreview
  (bind _owningplayer (Variables|Default|GetOwningPlayer))
  (bind _predictresult (Class|GameplayStatics|BlueprintPredictProjectilePathAdvanced (Utilities|Struct|MakePredictProjectilePathParams (Transformation|GetWorldLocation (Variables|Default|GetThrowingComponent)) (* (Math|Vector|GetForwardVector (Variables|/Game/GraveCrawlers/Entities/Character/BP_MainChar.BP_MainChar_C|GetFollowCamera _owningplayer)) (Variables|/Game/GraveCrawlers/Data/Blueprints/PDA_SlowAbility.PDA_SlowAbility_C|GetThrowForce (Variables|Default|GetSlowAbilityDataAsset))) true 0.0 2.0 true "ECC_GameTraceChannel3" "ObjectTypeQuery1" (Utilities|Array|MakeArray _owningplayer) 2e+01 0.0 "None" 5.0 false)))
  (Transformation|SetWorldLocation (Variables|Default|GetAbilityPreviewObject) (.location (Utilities|Array|Get(acopy) (.PathData (Utilities|Struct|BreakPredictProjectilePathResult _predictresult)) (Utilities|Array|LastIndex (.PathData (Utilities|Struct|BreakPredictProjectilePathResult _predictresult))))) false false))