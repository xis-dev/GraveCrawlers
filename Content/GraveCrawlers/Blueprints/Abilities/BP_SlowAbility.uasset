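; BP_SlowAbility is a timed area-of-effect actor that slows Enemy actors inside its box.
; Initialize stores radius, slow percent and duration, scales the mesh horizontally, starts an expiry timer and slows enemies already overlapping.
; Box overlaps halt and slow entering enemies, recording each applied slow in a map, and lift it on exit.
; Remove calls RemoveSlow for every valid map entry, which exits leave in place, then destroys the actor.
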(event OnComponentBeginOverlap(Box)
  (params (OverlappedComponent :type Primitive%20Component%20Object%20Reference) (OtherActor :type Actor%20Object%20Reference) (OtherComp :type Primitive%20Component%20Object%20Reference) (OtherBodyIndex :type Integer) (bFromSweep :type Boolean) (SweepResult :type Hit%20Result%20Structure%20%28by%20ref%29))
  (bind _asenemy (Utilities|Casting|CastToEnemy OtherActor))
  (CallFunction|SlowDownEnemy _asenemy))

(event OnComponentEndOverlap(Box)
  (params (OverlappedComponent :type Primitive%20Component%20Object%20Reference) (OtherActor :type Actor%20Object%20Reference) (OtherComp :type Primitive%20Component%20Object%20Reference) (OtherBodyIndex :type Integer))
  (bind _asenemy (Utilities|Casting|CastToEnemy OtherActor))
  (if (.ReturnValue (Utilities|Map|Find (Variables|Default|GetEnemiesAndCurrentSlowApplied) _asenemy))
    (Class|Enemy|RemoveSlow _asenemy (.Value (Utilities|Map|Find (Variables|Default|GetEnemiesAndCurrentSlowApplied) _asenemy)))))

(event EventBeginPlay
  (|CallParentFunction) ; This node is disabled and will not be called.\nDrag off pins to build functionality.
)

(event Collision|EventActorBeginOverlap
  (params (OtherActor :type Actor%20Object%20Reference))
  (|CallParentFunction OtherActor) ; This node is disabled and will not be called.\nDrag off pins to build functionality.
)

(event EventTick
  (params (DeltaSeconds :type Float%20%28single-precision%29))
  (|CallParentFunction DeltaSeconds) ; This node is disabled and will not be called.\nDrag off pins to build functionality.
)

(fn ConstructionScript
  (|CallParentFunction))

(fn Initialize
  (params (Radius :type Float%20%28double-precision%29) (SlowAmount :type Float%20%28double-precision%29) (Duration :type Float%20%28double-precision%29))
  (bind _output_get (Variables|Default|SetRadius Radius))
  (Variables|Default|SetSlowPercent SlowAmount)
  (bind _output_get_2 (Variables|Default|SetDuration Duration))
  (Utilities|Time|SetTimerbyEvent (EventDispatchers|CreateEvent :!event Remove) _output_get_2)
  (Transformation|SetRelativeScale3D (Variables|Default|GetStaticMesh) (Math|Vector|MakeVector _output_get _output_get (.z (Variables|/Script/Engine.SceneComponent|GetRelativeScale3D (Variables|Default|GetStaticMesh)))))
  (for _array_element (Collision|GetOverlappingActors (Variables|Default|GetBox) "/Script/Prototype1.Enemy" :!class /Script/Engine.PrimitiveComponent)
    (bind _asenemy (Utilities|Casting|CastToEnemy _array_element))
    (CallFunction|SlowDownEnemy _asenemy)))

(fn Remove
  (bind (_keypin _valuepin) (Utilities|Map|ForEachLoop(Map) (Variables|Default|GetEnemiesAndCurrentSlowApplied))
    (:then
      (Utilities|IsValid _keypin
        (:Is%20Valid
          (Class|Enemy|RemoveSlow _keypin _valuepin))))
    (:CompletedPin
      (Actor|DestroyActor))))

(fn SlowDownEnemy
  (params (Enemy :type Enemy%20Object%20Reference))
  (Components|Movement|StopMovementImmediately (Variables|/Script/Prototype1.GCCharacter|GetMovementComponent Enemy))
  (bind _returnvalue (Class|Enemy|ApplySlow Enemy (Variables|Default|GetSlowPercent)))
  (Utilities|Map|Add (Variables|Default|GetEnemiesAndCurrentSlowApplied) Enemy _returnvalue))