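; Candle actor that makes its three point lights flicker.
; A looping timer started on BeginPlay regularly picks a random target intensity.
; Tick smoothly interpolates from the current intensity of one light toward that target and applies the result to all three lights, keeping them in sync.
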(event Custom|Flicker
  (Variables|Default|SetIntensity (Math|Random|RandomFloatinRange 5.0 2e+01)))

(event EventBeginPlay
  (Utilities|Time|SetTimerbyEvent (delegate Custom|Flicker) 0.1 true))

(event Collision|EventActorBeginOverlap
  (params (OtherActor :type Actor%20Object%20Reference)))

(event EventTick
  (params (DeltaSeconds :type Float%20%28single-precision%29))
  (Rendering|Components|Light|SetIntensity (Variables|Default|GetPointLight1) (Math|Interpolation|FInterpTo (Variables|/Script/Engine.LightComponentBase|GetIntensity (Variables|Default|GetPointLight)) (Variables|Default|GetIntensity) DeltaSeconds 6.0)))

(fn ConstructionScript)