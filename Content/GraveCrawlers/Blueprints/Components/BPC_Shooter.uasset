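; Shooter component that handles hitscan firing, ammo, reloading and fire rate for the owner's current gun.
; Shoot line-traces from the muzzle to a target point, returns the hit actor for the caller, starts a cooldown timer and auto-reloads when empty.
; Reload cancels the cooldown and blocks shooting during a timed reload, with dispatchers announcing reloads and ammo changes.
; Damage is only stored here, never applied.
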(event Custom|ResetCanShoot
  (Variables|Default|SetbCanShoot true))

(event EventBeginPlay)

(event EventTick
  (params (DeltaSeconds :type Float%20%28single-precision%29)))

(fn Shoot
  (params (TargetDirection :type Vector))
  (bind _currentammo (Variables|WeaponStats|GetCurrentAmmo))
  (bind _shotcooldown (Variables|WeaponStats|GetShotCooldown))
  (if (Variables|Default|GetbCanShoot)
    (Variables|Default|SetbCanShoot false)
    (bind (_outhit _returnvalue) (Collision|LineTraceByChannel (Transformation|GetWorldLocation (Variables|/Game/GraveCrawlers/Blueprints/BP_Gun.BP_Gun_C|GetMuzzle (Variables|Default|GetCurrentGun))) TargetDirection "TraceTypeQuery4" false (Utilities|Array|MakeArray (Components|GetOwner)) "None"))
    (Default|ShotFired (Variables|Default|GetCurrentGun) _shotcooldown)
    (bind _returnvalue_2 (Utilities|Time|SetTimerbyEvent (EventDispatchers|CreateEvent :!event Custom|ResetCanShoot) _shotcooldown))
    (Variables|Default|SetResetShotTimer _returnvalue_2)
    (bind _result (Math|Integer|DecrementInt _currentammo)
      (:%20%20
        (if (<= _result 0)
          (CallFunction|Reload))
        (Default|CallAmmoUsed)
        (return _returnvalue (.hitactor _outhit) _currentammo)))
    (else
      (return false 0 (Variables|WeaponStats|GetCurrentAmmo)))))

(fn Reload
  (bind _reloadtime (Variables|WeaponStats|GetReloadTime))
  (Utilities|Time|ClearandInvalidateTimerbyHandle (Variables|Default|GetResetShotTimer))
  (if (< (Variables|WeaponStats|GetCurrentAmmo) (Variables|WeaponStats|GetMaxAmmoReserve))
    (if (Variables|Default|GetbCanReload)
      (Variables|Default|SetbCanReload false)
      (Variables|Default|SetbCanShoot false)
      (Default|CallReloaded _reloadtime)
      (Utilities|Time|SetTimerbyEvent (EventDispatchers|CreateEvent :!event ResetAmmo) _reloadtime))))

(fn GainAmmo
  (params (AmmoToAdd :type Integer))
  (bind _output_get (Variables|WeaponStats|SetMaxAmmoReserve (+ AmmoToAdd (Variables|WeaponStats|GetMaxAmmoReserve))))
  (bind _output_get_2 (Variables|WeaponStats|SetCurrentAmmo (Math|Integer|Clamp(Integer) (+ AmmoToAdd (Variables|WeaponStats|GetCurrentAmmo)) 0 _output_get)))
  (Default|CallAmmoUsed)
  (return _output_get_2 _output_get))

(fn Initialize
  (params (AmmoReserve :type Integer))
  (bind _output_get (Variables|WeaponStats|SetMaxAmmoReserve AmmoReserve))
  (bind _output_get_2 (Variables|WeaponStats|SetCurrentAmmo _output_get))
  (return _output_get_2))

(fn ResetAmmo
  (Variables|WeaponStats|SetCurrentAmmo (Variables|WeaponStats|GetMaxAmmoReserve))
  (Default|CallAmmoUsed)
  (Variables|Default|SetbCanShoot true)
  (Variables|Default|SetbCanReload true))

(fn SetFireRate
  (params (NewRate :type Float%20%28double-precision%29))
  (bind _output_get (Variables|WeaponStats|SetFireRate NewRate))
  (bind _output_get_2 (Variables|WeaponStats|SetShotCooldown (/ 1.0 _output_get)))
  (return _output_get _output_get_2))

(fn SetCurrentandMaxAmmo
  (params (Current :type Integer) (Max :type Integer))
  (bind _output_get (Variables|WeaponStats|SetMaxAmmoReserve Max))
  (Variables|WeaponStats|SetCurrentAmmo (Math|Integer|Clamp(Integer) Current 0 _output_get))
  (Default|CallAmmoManipulated))

(fn SetDamage
  (params (DamageValue :type Float%20%28double-precision%29))
  (bind _output_get (Variables|WeaponStats|SetDamage DamageValue))
  (return _output_get))