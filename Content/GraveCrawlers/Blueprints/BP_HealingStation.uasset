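; Healing station that restores the player's health from a limited pool while they stand inside its sphere, draining the pool as it heals.
; A looping timer does the healing, and the aura switches off when the pool empties.
; Leaving starts a cooldown timer, with separate logic to recharge the pool over time; re-entering cancels both.
; A larger visibility trigger shows a green pool bar widget, turned toward the camera by a timer rather than Tick.
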(event OnComponentBeginOverlap(Sphere)
  (params (OverlappedComponent :type Primitive%20Component%20Object%20Reference) (OtherActor :type Actor%20Object%20Reference) (OtherComp :type Primitive%20Component%20Object%20Reference) (OtherBodyIndex :type Integer) (bFromSweep :type Boolean) (SweepResult :type Hit%20Result%20Structure%20%28by%20ref%29))
  (bind _returnvalue (Game|GetPlayerCharacter 0))
  ;[0.15 0.15 0.15 0.5] HealingSphere
  (if (== OtherActor _returnvalue)
    (bind _asbp_main_char (Utilities|Casting|CastToBP_MainChar _returnvalue))
    (Variables|Default|SetCanDistributeHealth true)
    (Variables|Default|SetPlayerToDistributeTo _asbp_main_char)
    (CallFunction|StartHealingPlayer)
    (Utilities|Time|ClearandInvalidateTimerbyHandle (Variables|TimerHandles|GetCooldownTimerHandle))
    (Utilities|Time|ClearandInvalidateTimerbyHandle (Variables|TimerHandles|GetHealthRechargingTimerHandle))))

(event OnComponentEndOverlap(Sphere)
  (params (OverlappedComponent :type Primitive%20Component%20Object%20Reference) (OtherActor :type Actor%20Object%20Reference) (OtherComp :type Primitive%20Component%20Object%20Reference) (OtherBodyIndex :type Integer))
  ;[0.15 0.15 0.15 0.5] HealingSphere
  (if (== OtherActor (Game|GetPlayerCharacter 0))
    (CallFunction|StopHealingPlayer)
    (Variables|Default|SetPlayerToDistributeTo 0)
    (Variables|Default|SetCanDistributeHealth false)
    (bind _returnvalue (Utilities|Time|SetTimerbyEvent (EventDispatchers|CreateEvent :!event StartRecharging) (Variables|Timers|GetCooldownTime)))
    (Variables|TimerHandles|SetCooldownTimerHandle _returnvalue)))

(event OnComponentBeginOverlap(HealingBarVisibilityTrigger)
  (params (OverlappedComponent :type Primitive%20Component%20Object%20Reference) (OtherActor :type Actor%20Object%20Reference) (OtherComp :type Primitive%20Component%20Object%20Reference) (OtherBodyIndex :type Integer) (bFromSweep :type Boolean) (SweepResult :type Hit%20Result%20Structure%20%28by%20ref%29))
  ;[0.15 0.15 0.15 0.5] HealthBar Visibility Sphere
  (if (== OtherActor (Game|GetPlayerCharacter 0))
    (Utilities|ShowandStartOrientingHealthBar)))

(event OnComponentEndOverlap(HealingBarVisibilityTrigger)
  (params (OverlappedComponent :type Primitive%20Component%20Object%20Reference) (OtherActor :type Actor%20Object%20Reference) (OtherComp :type Primitive%20Component%20Object%20Reference) (OtherBodyIndex :type Integer))
  ;[0.15 0.15 0.15 0.5] HealthBar Visibility Sphere
  (if (== OtherActor (Game|GetPlayerCharacter 0))
    (Utilities|HideandStopOrientingHealthBar)))

(event EventBeginPlay
  (bind _healingbarvisibilitytrigger (Variables|Default|GetHealingBarVisibilityTrigger))
  (bind _aswbp_health_bar (Utilities|Casting|CastToWBP_HealthBar (UserInterface|GetWidget (Variables|Default|GetAvailableHealing))))
  (Variables|Default|SetHealthBarBP _aswbp_health_bar)
  (Default|ChangeHealthBarColour _aswbp_health_bar "(R=0.000000,G=1.000000,B=0.014251,A=1.000000)")
  ;[0.15 0.15 0.15 0.5] Find player to toggle healthbar visibility
  (CallFunction|Reset)
  (bind _outhits (Collision|MultiSphereTraceForObjects (Transformation|GetWorldLocation _healingbarvisibilitytrigger) "0, 0, 0" (.SphereRadius (Collision|GetComponentBounds _healingbarvisibilitytrigger)) (Utilities|Array|MakeArray "ObjectTypeQuery3") false 0 "None"))
  (bind _array_element (Utilities|Array|ForEachLoopwithBreak _outhits :!label _label)
    (:LoopBody
      (if (== (.hitactor _array_element) (Game|GetPlayerCharacter 0))
        (Utilities|ShowandStartOrientingHealthBar)
        (goto _label Break)))))

(event Collision|EventActorBeginOverlap
  (params (OtherActor :type Actor%20Object%20Reference)))

(fn ConstructionScript
  (Variables|Amounts|SetCurrentAmount (Variables|Amounts|GetMaxAmount))
  (bind _aswbp_health_bar (Utilities|Casting|CastToWBP_HealthBar (UserInterface|GetWidget (Variables|Default|GetAvailableHealing))))
  (Default|ChangeHealthBarColour _aswbp_health_bar "(R=0.000000,G=1.000000,B=0.014251,A=1.000000)"))

(fn DeductCurrentAmount
  (params (Amount :type Float%20%28double-precision%29))
  (Variables|Amounts|SetCurrentAmount (Math|Float|Clamp(Float) (- (Variables|Amounts|GetCurrentAmount) Amount) 0.0 (Variables|Amounts|GetMaxAmount))))

(fn Reset
  (Variables|Amounts|SetCurrentAmount (Variables|Amounts|GetMaxAmount))
  (Collision|SetCollisionEnabled (Variables|Default|GetSphere) "QueryOnly")
  (Variables|Default|SetOnCooldown false))

(fn GiveHealthtoPlayer)

(fn OrientHealthBartoPlayer
  (bind _availablehealing (Variables|Default|GetAvailableHealing))
  (Transformation|SetWorldRotation _availablehealing (Math|Rotator|FindLookatRotation (Transformation|GetWorldLocation _availablehealing) (Camera|GetCameraLocation (Game|GetPlayerCameraManager 0))) false false))

(fn ShowHealthBar)

(fn HideHealthBar)

(fn StartHealingPlayer
  (CallFunction|HealPlayer)
  (bind _returnvalue (Utilities|Time|SetTimerbyEvent (EventDispatchers|CreateEvent :!event HealPlayer) (Variables|Timers|GetHealthDistributionTimerTick) true))
  (Variables|TimerHandles|SetHealthDistributionTimerHandle _returnvalue))

(fn HealPlayer
  (bind _healthdistributiontimertick (Variables|Timers|GetHealthDistributionTimerTick))
  (bind _playertodistributeto (Variables|Default|GetPlayerToDistributeTo))
  (bind _healthtodistributepersecond (Variables|Amounts|GetHealthToDistributePerSecond))
  (bind _healingaura (Variables|Default|GetHealingAura))
  (bind _returnvalue (* _healthtodistributepersecond _healthdistributiontimertick))
  (bind _healthcomponent_ (Variables|/Game/GraveCrawlers/Entities/Character/BP_MainChar.BP_MainChar_C|GetHealthComponent%20 _playertodistributeto))
  (if (> (Variables|Amounts|GetCurrentAmount) 0.0)
    (if (< (Variables|/Script/Prototype1.HealthComponent|GetCurrentHealth _healthcomponent_) (Variables|/Script/Prototype1.HealthComponent|GetMaxHealth _healthcomponent_))
      (Class|HealthComponent|Heal _healthcomponent_ _returnvalue)
      (CallFunction|DeductCurrentAmount _returnvalue)
      (Progress|SetPercent (Variables|/Game/GraveCrawlers/UI/WBP_HealthBar.WBP_HealthBar_C|GetHealthBar (Variables|Default|GetHealthBarBP)) (Math|Float|SafeDivide (Variables|Amounts|GetCurrentAmount) (Variables|Amounts|GetMaxAmount))))
    (elif (not (Variables|Default|GetHealthIsFullyDepleted))
      (Variables|Default|SetHealthIsFullyDepleted true)
      (Components|Activation|Deactivate _healingaura)
      (Rendering|SetVisibility _healingaura false false))))

(fn StopHealingPlayer
  (Utilities|Time|ClearandInvalidateTimerbyHandle (Variables|TimerHandles|GetHealthDistributionTimerHandle)))

(fn IncrementCurrentAmount
  (params (Amount :type Float%20%28double-precision%29))
  (Variables|Amounts|SetCurrentAmount (Math|Float|Clamp(Float) (+ Amount (Variables|Amounts|GetCurrentAmount)) 0.0 (Variables|Amounts|GetMaxAmount))))

(fn StartRecharging
  (bind _healingaura (Variables|Default|GetHealingAura))
  (if (Variables|Default|GetHealthIsFullyDepleted)
    (Components|Activation|Activate _healingaura false)
    (Rendering|SetVisibility _healingaura true false))
  (Variables|Default|SetHealthIsFullyDepleted false)
  (bind _returnvalue (Utilities|Time|SetTimerbyEvent (EventDispatchers|CreateEvent :!event RechargeHealth) (Variables|Timers|GetHealthDistributionTimerTick) true))
  (Variables|TimerHandles|SetHealthRechargingTimerHandle _returnvalue))

(fn RechargeHealth
  (if (>= (Variables|Amounts|GetCurrentAmount) (Variables|Amounts|GetMaxAmount))
    (Utilities|Time|ClearandInvalidateTimerbyHandle (Variables|TimerHandles|GetHealthRechargingTimerHandle))
    (else
      (CallFunction|IncrementCurrentAmount (* (Variables|Amounts|GetHealthToRechargePerSecond) (Variables|Timers|GetHealthDistributionTimerTick)))
      (Progress|SetPercent (Variables|/Game/GraveCrawlers/UI/WBP_HealthBar.WBP_HealthBar_C|GetHealthBar (Variables|Default|GetHealthBarBP)) (Math|Float|SafeDivide (Variables|Amounts|GetCurrentAmount) (Variables|Amounts|GetMaxAmount))))))