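; Player controller for GraveCrawlers that links the main character, game mode and main HUD across pause and death.
; It creates the HUD, adds the input mapping and updates widgets from game states returned or broadcast by the game mode.
; The pause input either pauses or, if already paused, calls a go-back event.
; Death events clear the game, then trigger game over with a high score persisted to a save slot.
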(event Input|EnhancedActionEvents|EnhancedInputActionIA_Pause
  (params (ActionValue :type Boolean) (ElapsedSeconds :type Float%20%28double-precision%29) (TriggeredSeconds :type Float%20%28double-precision%29) (InputAction :type Input%20Action%20Object%20Reference :default "/Game/GraveCrawlers/Inputs/IA_Pause.IA_Pause"))
  ;[0.15 0.15 0.15 0.5] Pausing
  (:Started
    (bind _gamemodeobject (Variables|Default|GetGameModeObject)
      (:then
        (bind _gamestate (Default|GetGameState _gamemodeobject))
        (if (Utilities|Enum|Equal(Enum) _gamestate "NewEnumerator1")
          (Default|CallGoBackWhilePaused)
          (else
            (CallFunction|PauseGame))))
      (:else))))

(event EventBeginPlay
  (bind _returnvalue (UserInterface|CreateWidget "/Game/GraveCrawlers/UI/WBP_MainHUD.WBP_MainHUD_C"))
  (UserInterface|Viewport|AddtoViewport _returnvalue 0)
  (Variables|Default|SetMainWidget _returnvalue)
  (Input|AddMappingContext (PlayerController|LocalPlayerSubsystems|GetEnhancedInputLocalPlayerSubsystem self) "/Game/GraveCrawlers/Inputs/IMC_Base.IMC_Base" 0 "(bIgnoreAllPressedKeysUntilRelease=True,bForceImmediately=False,bNotifyUserSettings=False)")
  (bind _asbp_main_game_mode (Utilities|Casting|CastToBP_MainGameMode (Game|GetGameMode)))
  (bind _output_get (Variables|Default|SetGameModeObject _asbp_main_game_mode))
  (EventDispatchers|BindEventtoOnGameResumed _output_get (EventDispatchers|CreateEvent :!event GameResumed)))

(event EventPossess
  (params (PossessedPawn :type Pawn%20Object%20Reference))
  (|CallParentFunction PossessedPawn)
  (bind _asbp_main_char (Utilities|Casting|CastToBP_MainChar PossessedPawn))
  (bind _output_get (Variables|Default|SetPossessedPlayer _asbp_main_char))
  (EventDispatchers|BindEventtoOnPlayerFinishDeath _output_get (EventDispatchers|CreateEvent :!event OnPlayerFinishDeath))
  (EventDispatchers|BindEventtoOnPlayerStartDeath _output_get (EventDispatchers|CreateEvent :!event OnPlayerStartDeath)))

(fn ConstructionScript)

(fn PauseGame
  (bind _gamestateout (Default|PauseGame (Variables|Default|GetGameModeObject)))
  (Default|WidgetbyGameState (Variables|Default|GetMainWidget) _gamestateout))

(fn GameResumed
  (params (GameState :type E_GameState%20Enum :default "NewEnumerator0"))
  (bind _mainwidget (Variables|Default|GetMainWidget)
    (:then
      (Default|WidgetbyGameState _mainwidget GameState))
    (:else)))

(fn OnPlayerFinishDeath
  (params (Player :type BP%20Main%20Char%20Object%20Reference))
  (bind _score (Variables|/Script/Prototype1.MainPlayer|GetScore Player))
  (bind _gamemodeobject (Variables|Default|GetGameModeObject)
    (:then
      (bind _gamestateout (Default|GameOver _gamemodeobject))
      (bind _highscoreout (CallFunction|SaveHighScore _score))
      (bind _mainwidget (Variables|Default|GetMainWidget)
        (:then
          (Default|WidgetbyGameState _mainwidget _gamestateout)
          (Default|GameOver _mainwidget _score _highscoreout))
        (:else)))
    (:else)))

(fn ResumeGame
  (bind _gamestateout (Default|ResumeGame (Variables|Default|GetGameModeObject)))
  (bind _mainwidget (Variables|Default|GetMainWidget)
    (:then
      (Default|WidgetbyGameState _mainwidget _gamestateout))
    (:else)))

(fn SaveHighScore
  (params (Score :type Integer))
  (bind _returnvalue (SaveGame|LoadGamefromSlot "SAVE_Gameplay"))
  (Utilities|IsValid _returnvalue
    (:Is%20Valid
      (bind _asbp_gameplay_save_game (Utilities|Casting|CastToBP_GameplaySaveGame _returnvalue)))
    (:Is%20Not%20Valid
      (bind _returnvalue_2 (SaveGame|CreateSaveGameObject "/Game/GraveCrawlers/Blueprints/BP_GameplaySaveGame.BP_GameplaySaveGame_C"))))
  (bind _output_get (Variables|/Game/GraveCrawlers/Blueprints/BP_GameplaySaveGame.BP_GameplaySaveGame_C|SetHighScore (select (Utilities|IsValid _returnvalue) _asbp_gameplay_save_game _returnvalue_2) (select (> Score (Variables|/Game/GraveCrawlers/Blueprints/BP_GameplaySaveGame.BP_GameplaySaveGame_C|GetHighScore (select (Utilities|IsValid _returnvalue) _asbp_gameplay_save_game _returnvalue_2))) Score (Variables|/Game/GraveCrawlers/Blueprints/BP_GameplaySaveGame.BP_GameplaySaveGame_C|GetHighScore (select (Utilities|IsValid _returnvalue) _asbp_gameplay_save_game _returnvalue_2)))))
  (SaveGame|SaveGametoSlot (select (Utilities|IsValid _returnvalue) _asbp_gameplay_save_game _returnvalue_2) "SAVE_Gameplay")
  (return _output_get))

(fn OnPlayerStartDeath
  (Default|ClearGame (Variables|Default|GetGameModeObject))
  (bind _mainwidget (Variables|Default|GetMainWidget)
    (:then
      (Default|PlayerDeath _mainwidget))
    (:else)))