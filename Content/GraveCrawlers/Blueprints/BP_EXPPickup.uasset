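; BP_EXPPickup is an experience pickup that grants EXP to the main character, built on a parent pickup class.
; Drop stores the amount of experience the pickup carries.
; ApplyPickup runs the parent logic, then casts the target to BP_MainChar and passes that amount to TryGiveExp.
; Pickup defers entirely to the parent, and the event graph holds no active logic.
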(event EventBeginPlay)

(event Collision|EventActorBeginOverlap
  (params (OtherActor :type Actor%20Object%20Reference)))

(event EventTick
  (params (DeltaSeconds :type Float%20%28single-precision%29))
  (|CallParentFunction DeltaSeconds) ; This node is disabled and will not be called.\nDrag off pins to build functionality.
)

(fn ConstructionScript
  (|CallParentFunction))

(fn ApplyPickup
  (params (ActorToApplyTo :type Actor%20Object%20Reference))
  (|CallParentFunction ActorToApplyTo)
  (bind _asbp_main_char (Utilities|Casting|CastToBP_MainChar ActorToApplyTo))
  (Default|TryGiveExp _asbp_main_char (Variables|Default|GetEXPAmount)))

(fn Pickup
  (params (PickingActor :type Actor%20Object%20Reference))
  (|CallParentFunction PickingActor))

(fn Drop
  (params (ExpAmount :type Float%20%28double-precision%29))
  (Variables|Default|SetEXPAmount ExpAmount))