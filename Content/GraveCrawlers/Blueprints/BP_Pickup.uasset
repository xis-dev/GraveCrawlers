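; Base pickup actor that spins its sphere each tick and flies to player 0 when picked.
; Pickup fires OnPicked, whose Movement timeline lerps the actor from its current location toward the player.
; A CompareDistance success or the timeline's end calls ApplyPickup, empty here, then destroys the actor.
; CompareDistance's radius test is left unconnected, and CanBePicked is only ever cleared, never read.
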(event Custom|OnPicked
  (params (PickingActor :type Actor%20Object%20Reference))
  (bind _lerpalpha (Timeline|Movement Play)
    (:Update
      (Transformation|SetActorLocation (Math|Vector|Lerp(Vector) (Transformation|GetActorLocation) (Transformation|GetActorLocation (Game|GetPlayerCharacter 0)) _lerpalpha) false false)
      (if (|CompareDistance)
        (Variables|Default|SetbCanBePicked false)
        (Utilities|FlowControl|Sequence
          (:then_0
            (Timeline|Movement Stop))
          (:then_1
            (CallFunction|ApplyPickup PickingActor :!label _label)
            (Actor|DestroyActor)))))
    (:Finished
      (goto _label))))

(event EventTick
  (params (DeltaSeconds :type Float%20%28single-precision%29))
  (|RotateSphere DeltaSeconds DeltaSeconds))

(fn ConstructionScript)

(fn Pickup
  (params (PickingActor :type Actor%20Object%20Reference))
  (CallFunction|OnPicked PickingActor))

(fn ApplyPickup
  (params (ActorToApplyTo :type Actor%20Object%20Reference)))

(fn StopTryingtoPickup
  (Variables|Default|SetbCanBePicked false))