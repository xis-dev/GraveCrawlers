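; BP_SingleCandle is a candle actor whose point light flickers.
; A looping timer started on BeginPlay picks a new random target intensity several times a second.
; Tick interpolates the light's current intensity toward that target, smoothing the random steps into a soft flicker.
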(event Custom|Flicker
  (Variables|Default|SetIntensity (Math|Random|RandomFloatinRange 3.0 8.0)))

(event EventBeginPlay
  (Variables|Default|SetIntensity (Variables|/Script/Engine.LightComponentBase|GetIntensity (Variables|Default|GetPointLight)))
  (Utilities|Time|SetTimerbyEvent (delegate Custom|Flicker) 0.1 true))

(event Collision|EventActorBeginOverlap
  (params (OtherActor :type Actor%20Object%20Reference)))

(event EventTick
  (params (DeltaSeconds :type Float%20%28single-precision%29))
  (bind _pointlight (Variables|Default|GetPointLight))
  (Rendering|Components|Light|SetIntensity _pointlight (Math|Interpolation|FInterpTo (Variables|/Script/Engine.LightComponentBase|GetIntensity _pointlight) (Variables|Default|GetIntensity) DeltaSeconds 5.0)))

(fn ConstructionScript)