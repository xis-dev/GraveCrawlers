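; Main game mode for GraveCrawlers, managing game state, two switchable play modes, wave spawning and player respawn.
; SetGameState records previous states and pauses or resumes the game, input mode and cursor for playing, paused, upgrading and game-over states.
; StartGame begins timed waves through WaveSystem.
; The second mode drains player health non-lethally on a timer and calls SwapGameMode when the damage call returns a near-minimum value.
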(event Custom|RespawnPlayer
  (params (Player :type Character%20Object%20Reference))
  (bind _returnvalue (Game|SpawnActorfromClass (Utilities|GetClass Player) (Variables|Default|GetSpawnTransform) "AdjustIfPossibleButAlwaysSpawn" "MultiplyWithRoot" 0 0))
  (Utilities|IsValid _returnvalue
    (:Is%20Valid
      (Input|EnableInput _returnvalue 0)
      (Default|CallPlayerRespawned)
      (GameState|SetGameState "NewEnumerator0")
      (CallFunction|StartGame))))

(event EventBeginPlay
  (|CallParentFunction))

(fn ConstructionScript)

(fn IntoSecondMode
  (Default|CallOnChangedtoSecondMode))

(fn OutOfSecondMode
  (Default|CallOnChangedtoFirstMode))

(fn GameOver
  (bind _gamestateout (GameState|SetGameState "NewEnumerator4"))
  (return _gamestateout))

(fn GetGameState
  (return (Variables|GameVariables|GetCurrentGameState)))

(fn SetGameState
  (params (GameState :type E_GameState%20Enum :default "NewEnumerator0"))
  (if (or (Utilities|Enum|Equal(Enum) (Variables|GameVariables|GetCurrentGameState) "NewEnumerator0") (Utilities|Enum|Equal(Enum) (Variables|GameVariables|GetCurrentGameState) "NewEnumerator3"))
    (Variables|GameVariables|SetPreviousGameplayTypeState (Variables|GameVariables|GetCurrentGameState)))
  (Variables|GameVariables|SetPreviousGameState (Variables|GameVariables|GetCurrentGameState))
  (bind _output_get (Variables|GameVariables|SetCurrentGameState GameState))
  (switch Utilities|FlowControl|Switch|SwitchonE_GameState _output_get
    (:NewEnumerator0
      (Utilities|Resume :!label _label))
    (:NewEnumerator1
      (Utilities|Pause :!label _label_2))
    (:NewEnumerator2
      (goto _label_2))
    (:NewEnumerator3
      (goto _label))
    (:NewEnumerator4
      (goto _label_2)))
  (return _output_get))

(fn PauseGame
  (bind _gamestateout (GameState|SetGameState "NewEnumerator1"))
  (return _gamestateout))

(fn ResumeGame
  (if (Utilities|Enum|Equal(Enum) (Variables|GameVariables|GetCurrentGameState) "NewEnumerator1")
    (bind _gamestateout (GameState|SetGameState (Variables|GameVariables|GetPreviousGameState)))
    (Default|CallOnGameResumed _gamestateout)
    (return _gamestateout)))

(fn ResumetoGameplay
  ;[0.01553 0.03494 0.15 0.5] TODO: Temp func, remove
  (GameState|SetGameState (Variables|GameVariables|GetPreviousGameplayTypeState)))

(fn ContinueGame
  (bind _wavesystem (Variables|Default|GetWaveSystem))
  (Class|WaveSystem|StartWave _wavesystem 32)
  (bind _returnvalue (Utilities|Time|SetTimerbyEvent (EventDispatchers|CreateEvent :!event StartNewWave) (Variables|/Script/Prototype1.WaveConfigDataAsset|GetWaveInterval (Variables|/Script/Prototype1.WaveSystem|GetWaveSystemConfig _wavesystem)) true))
  (Variables|WaveConfig|SetWaveTimerHandle _returnvalue))

(fn StartNewWave
  (Class|WaveSystem|StartWave (Variables|Default|GetWaveSystem) 32))

(fn StartGame
  (|CallParentFunction)
  (GameState|SetGameState "NewEnumerator0")
  (Game|ContinueGame))

(fn SwapGameMode
  (params (Player :type BP%20Main%20Char%20Object%20Reference))
  (bind _currentgamestate (Variables|GameVariables|GetCurrentGameState))
  (if (not (or (Utilities|Enum|Equal(Enum) _currentgamestate "NewEnumerator1") (Utilities|Enum|Equal(Enum) _currentgamestate "NewEnumerator2")))
    (if (Utilities|Enum|Equal(Enum) _currentgamestate "NewEnumerator0")
      (bind _gamestateout (GameState|SetGameState "NewEnumerator3"))
      (CallFunction|IntoSecondMode)
      (CallFunction|StartDamagingPlayerinSecondMode Player)
      (return _gamestateout)
      (else
        (bind _gamestateout_2 (GameState|SetGameState "NewEnumerator0"))
        (CallFunction|OutOfSecondMode)
        (CallFunction|StopDamagingPlayer)
        (return _gamestateout_2)))))

(fn StartDamagingPlayerinSecondMode
  (params (Player :type BP%20Main%20Char%20Object%20Reference))
  (Variables|SecondModeDamaging|SetPlayerToDamage Player)
  (CallFunction|DamagePlayer)
  (Utilities|Time|ClearandInvalidateTimerbyHandle (Variables|SecondModeDamaging|GetDamagePlayerTimerHandle))
  (Utilities|Time|SetTimerbyEvent (EventDispatchers|CreateEvent :!event DamagePlayer) (Variables|SecondModeDamaging|GetSecondModeDamagingTimerTick) true))

(fn StopDamagingPlayer
  (Utilities|Time|ClearandInvalidateTimerbyHandle (Variables|SecondModeDamaging|GetDamagePlayerTimerHandle))
  (Variables|SecondModeDamaging|SetPlayerToDamage 0))

(fn DamagePlayer
  (bind _playertodamage (Variables|SecondModeDamaging|GetPlayerToDamage)
    (:then
      (bind _returnvalue (Class|HealthComponent|DealNonLethalDamage (Variables|/Game/GraveCrawlers/Entities/Character/BP_MainChar.BP_MainChar_C|GetHealthComponent%20 _playertodamage) (* (Variables|/Script/Prototype1.GameConfigDataAsset|GetHealthLossRateInSecondMode (Variables|GameVariables|GetGameConfig)) (Variables|SecondModeDamaging|GetSecondModeDamagingTimerTick)) 0))
      (if (<= _returnvalue 1.1)
        (bind _gamestateout (GameState|SwapGameMode))
        (Development|PrintString (Utilities|String|EnumtoString _gamestateout))))
    (:else)))

(fn ClearGame
  (Utilities|Time|ClearandInvalidateTimerbyHandle (Variables|WaveConfig|GetWaveTimerHandle))
  (Class|AIManager|Clear (Variables|Default|GetAIManager)))