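; Lit torch Blueprint that makes its point light flicker.
; BeginPlay picks a random base intensity and starts a fast looping timer, which repeatedly sets a new random target scaled around that base.
; Tick eases the light toward the latest target with FInterpTo, smoothing the jumps, and the random base gives each instance its own brightness.
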(event Custom|FlicketStrong
  (bind _base_intensity (Variables|Default|GetBase%20Intensity))
  (Variables|Default|SetTarget%20Intensity (Math|Random|RandomFloatinRange (* _base_intensity 0.4) (* _base_intensity 1.3))))

(event EventBeginPlay
  (Variables|Default|SetBase%20Intensity (Math|Random|RandomFloatinRange 0.0 2e+02))
  (Utilities|Time|SetTimerbyEvent (delegate Custom|FlicketStrong) 0.1 true))

(event EventTick
  (params (DeltaSeconds :type Float%20%28single-precision%29))
  (bind _pointlightcomponent (Variables|Default|GetPointLightComponent))
  (Rendering|Components|Light|SetIntensity _pointlightcomponent (Math|Interpolation|FInterpTo (Variables|/Script/Engine.LightComponentBase|GetIntensity _pointlightcomponent) (Variables|Default|GetTarget%20Intensity) DeltaSeconds 2.0)))

(fn ConstructionScript)